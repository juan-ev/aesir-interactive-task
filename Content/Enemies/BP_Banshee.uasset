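; BP_Banshee is an enemy drawn as a Paper2D flipbook that billboards toward the player camera every tick, rotating only in yaw.
; Taking damage runs a timeline that tints the sprite from dark teal back to white.
; A collision overlap calls OnDiedEvent, and the bound OnDied handler plays the death flipbook once, then destroys the actor when it finishes.
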(event `self.ReceiveBeginPlay`
  (add `self.OnDied` (delegate `OnDied_Event`)))

(event `OnDied_Event`
  (bind _paperflipbook (`self.PaperFlipbook`))
  (`PaperFlipbookComponent.SetLooping` _paperflipbook false)
  (`PaperFlipbookComponent.SetFlipbook` _paperflipbook "/Game/Enemies/Sprites/PF_Banshee_Die.PF_Banshee_Die")
  (`PaperFlipbookComponent.PlayFromStart` _paperflipbook)
  (add `PaperFlipbookComponent.OnFinishedPlaying` _paperflipbook (delegate `OnFinishedPlaying`)))

(event `OnFinishedPlaying`
  (`self.K2_DestroyActor`))

(event `self.ReceiveTick`
  (params (DeltaSeconds :type "Float (single-precision)"))
  (`self.ApplyBillboard`))

(event `self.ReceiveAnyDamage`
  (params (Damage :type "Float (single-precision)") (DamageType :type "DamageType Object Reference") (InstigatedBy :type "Controller Object Reference") (DamageCauser :type "Actor Object Reference"))
  (bind _paperflipbook (`self.PaperFlipbook`))
  (bind (_direction _value) (`Timeline|DamageFeedback` :!via `PlayFromStart`)
    (:`Update`
      (`PaperFlipbookComponent.SetSpriteColor` _paperflipbook (`KismetMathLibrary.LinearColorLerp` (struct :`G` 0.207622 :`B` 0.219791 :`A` 1.0) (struct :`R` 1.0 :`G` 1.0 :`B` 1.0 :`A` 1.0) _value)))
    (:`Finished`
      (`PaperFlipbookComponent.SetSpriteColor` _paperflipbook (struct :`R` 1.0 :`G` 1.0 :`B` 1.0 :`A` 1.0)))))

(event `self.Collision.OnComponentBeginOverlap`
  (params (OverlappedComponent :type "PrimitiveComponent Object Reference") (OtherActor :type "Actor Object Reference") (OtherComp :type "PrimitiveComponent Object Reference") (OtherBodyIndex :type Integer) (bFromSweep :type Boolean) (SweepResult :type "HitResult Structure (by ref)"))
  (`self.OnDied_Event`))

(fn `ApplyBillboard`
  (`SceneComponent.K2_SetWorldRotation` (`self.PaperFlipbook`) (`KismetMathLibrary.Conv_VectorToRotator` (`KismetMathLibrary.GreaterGreater_VectorRotator` (`KismetMathLibrary.Normal` (* (- (`PlayerCameraManager.GetCameraLocation` (`GameplayStatics.GetPlayerCameraManager` 0)) (`SceneComponent.K2_GetComponentLocation` (`self.PaperFlipbook`))) (1.0 1.0 0.0))) (struct :`Yaw` 90.0))) false false))

(fn `UserConstructionScript`)